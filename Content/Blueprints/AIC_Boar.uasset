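; AIC_Boar is the AI controller for the boar enemy character, driving its movement.
; On possession it casts the pawn to BP_Boar and caches the reference.
; Every tick it calls the boar's own Move function, skipping it while the boar is dead or receiving damage.
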(event `self.ReceivePossess`
  (params (PossessedPawn :type "Pawn Object Reference"))
  (bind _asbp_boar (cast `/Game/Blueprints/BP_Boar` PossessedPawn))
  (set `self.BP_Boar_Ref` _asbp_boar))

(event `self.ReceiveTick`
  (params (DeltaSeconds :type "Float (single-precision)"))
  (bind _bp_boar_ref (`self.BP_Boar_Ref`)
    (:`then`
      (if (not (`/Game/Blueprints/BP_Enemy.IsDead` _bp_boar_ref))
        (if (not (`/Game/Blueprints/BP_Enemy.IsReceivingDamage` _bp_boar_ref))
          (`/Game/Blueprints/BP_Boar.Move` _bp_boar_ref))))
    (:`else`)))

(fn `UserConstructionScript`)