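; AI controller for the skeleton enemy that drives its movement while it is free to act.
; On possession it casts the pawn to BP_Skeleton and caches the reference.
; Each tick it calls the skeleton's own Move function unless the pawn is dead, receiving damage or attacking, leaving the movement logic in the pawn rather than using a behavior tree.
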(event `self.ReceivePossess`
  (params (PossessedPawn :type "Pawn Object Reference"))
  (bind _asbp_skeleton (cast `/Game/Blueprints/BP_Skeleton` PossessedPawn))
  (set `self.BP_Skeleton_Ref` _asbp_skeleton))

(event `self.ReceiveTick`
  (params (DeltaSeconds :type "Float (single-precision)"))
  (bind _bp_skeleton_ref (`self.BP_Skeleton_Ref`)
    (:`then`
      (if (not (`/Game/Blueprints/BP_Enemy.IsDead` _bp_skeleton_ref))
        (if (not (`/Game/Blueprints/BP_Enemy.IsReceivingDamage` _bp_skeleton_ref))
          (if (not (`/Game/Blueprints/BP_Skeleton.IsAttacking` _bp_skeleton_ref))
            (`/Game/Blueprints/BP_Skeleton.Move` _bp_skeleton_ref)))))
    (:`else`)))

(fn `UserConstructionScript`)