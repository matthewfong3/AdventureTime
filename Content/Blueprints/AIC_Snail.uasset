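; AIC_Snail is the AI controller for BP_Snail enemies, driving their constant forward crawl.
; On possess it casts and caches the snail pawn.
; Each tick it calls the snail's MoveForward while the snail is valid, not dead and not receiving damage, with no behavior tree or navigation.
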(event `self.ReceivePossess`
  (params (PossessedPawn :type "Pawn Object Reference"))
  (bind _asbp_snail (cast `/Game/Blueprints/BP_Snail` PossessedPawn))
  (set `self.BP_Snail_Ref` _asbp_snail))

(event `self.ReceiveTick`
  (params (DeltaSeconds :type "Float (single-precision)"))
  (bind _bp_snail_ref (`self.BP_Snail_Ref`)
    (:`then`
      (if (not (`/Game/Blueprints/BP_Enemy.IsDead` _bp_snail_ref))
        (if (not (`/Game/Blueprints/BP_Enemy.IsReceivingDamage` _bp_snail_ref))
          (`/Game/Blueprints/BP_Snail.MoveForward` _bp_snail_ref))))
    (:`else`)))

(fn `UserConstructionScript`)