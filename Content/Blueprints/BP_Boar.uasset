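; Paper2D boar enemy that turns around at ledges, walls and other enemies, and damages the player on contact.
; An attack-range volume switches it between walking and faster running, with Tick updating speed and flipbook.
; Taking damage interrupts the attack with a hit flipbook, timeline-faded red material flash, sound and brief hitstop via custom time dilation.
; On death it flickers, disables capsule collision and is destroyed after a delay.
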(event `self.ReceiveBeginPlay`
  ; Create a dynamic material instance and save a reference to it for the Trigger Sprite Flash Effect. Initialize health
  (bind _returnvalue (`PrimitiveComponent.CreateDynamicMaterialInstance` (`self.Sprite`) 0 null "None"))
  (set `self.DynamicSpriteMaterialRef` _returnvalue)
  (set `self.Health` 200.0))

(event `TriggerSpriteFlashEffect`
  (params (FlashMultiplier :type "Float (single-precision)" :default 1.0) (FlashColor :type "LinearColor Structure" :default (struct :`R` 1.0 :`A` 1.0)) (PlayRate :type "Float (single-precision)" :default 5.0))
  ; Trigger Sprite Flash Effect
  ;; Set the dynamic sprite material instance params to the event's input params
  (`MaterialInstanceDynamic.SetScalarParameterValue` (`self.DynamicSpriteMaterialRef`) "FlashMultiplier" FlashMultiplier)
  (`MaterialInstanceDynamic.SetVectorParameterValue` (`self.DynamicSpriteMaterialRef`) "FlashColor" FlashColor)
  ;; Set the play rate for the timeline of our Fade Out Effect and use the alpha value to smooth lerp the FlashMultiplier value
  (`TimelineComponent.SetPlayRate` (`self.FadeOutEffect`) PlayRate)
  (bind (_direction _alpha) (`Timeline|FadeOutEffect` :!via `PlayFromStart`)
    (:`Update`
      (`MaterialInstanceDynamic.SetScalarParameterValue` (`self.DynamicSpriteMaterialRef`) "FlashMultiplier" (`KismetMathLibrary.Lerp` 0.0 FlashMultiplier _alpha)))))

(event `Move`
  ; Allows boar to move
  (`self.AddMovementInput` (`self.GetActorForwardVector`)))

(event `self.ReceiveAnyDamage`
  (params (Damage :type "Float (single-precision)") (DamageType :type "DamageType Object Reference") (InstigatedBy :type "Controller Object Reference") (DamageCauser :type "Actor Object Reference"))
  ; Apply incoming damage
  ;; Overwrite IsAttacking state when receiving damage
  (set `self.IsAttacking` false)
  ;; Trigger sprite flash effect and apply hitstop effect
  (`self.TriggerSpriteFlashEffect` 1.0 (struct :`R` 1.0 :`A` 1.0) 3.0)
  (`self.StartHitstop` 0.05)
  (`GameplayStatics.PlaySound2D` "/Game/Sounds/damage1.damage1" 0.15 1.0 0.0 null null)
  (set `self.Health` (- (`self.Health`) Damage))
  (set `self.IsReceivingDamage` true)
  (if (<= (`self.Health`) 0.0)
    ;; Boar == dead, set flipbook, looping, start sprite flicker effect, disable collision, play sound. After delay, destroy actor
    (set `self.IsDead` true)
    (`PaperFlipbookComponent.SetFlipbook` (`self.Sprite`) "/Game/Assets/Mobs/Boar/Flipbooks/FB_Boar_Hit.FB_Boar_Hit")
    (`PaperFlipbookComponent.SetLooping` (`self.Sprite`) false)
    (`self.StartSpriteFlickerEffect`)
    (`PrimitiveComponent.SetCollisionEnabled` (`self.CapsuleComponent`) "NoCollision")
    (`GameplayStatics.PlaySound2D` "/Game/Sounds/enemy_death.enemy_death" 1.0 1.0 0.0 null null)
    (`KismetSystemLibrary.Delay` 1.5)
    (`self.K2_DestroyActor`)
    (else
      ;; Boar != dead, set flipbook, looping
      (`PaperFlipbookComponent.SetFlipbook` (`self.Sprite`) "/Game/Assets/Mobs/Boar/Flipbooks/FB_Boar_Hit.FB_Boar_Hit")
      (`PaperFlipbookComponent.SetLooping` (`self.Sprite`) false))))

(event `self.Sprite.OnFinishedPlaying`
  (bind _sprite (`self.Sprite`))
  ; When boar finishes playing Hit animation, reset flipbook animation, looping
  (if (not (`self.IsDead`))
    (if (`self.IsReceivingDamage`)
      (set `self.IsReceivingDamage` false)
      (`PaperFlipbookComponent.SetFlipbook` _sprite "/Game/Assets/Mobs/Boar/Flipbooks/FB_Boar_Walk.FB_Boar_Walk")
      (`PaperFlipbookComponent.SetLooping` _sprite true)
      (`PaperFlipbookComponent.Play` _sprite))))

(event `self.CollisionSphere.OnComponentBeginOverlap`
  (params (OverlappedComponent :type "PrimitiveComponent Object Reference") (OtherActor :type "Actor Object Reference") (OtherComp :type "PrimitiveComponent Object Reference") (OtherBodyIndex :type Integer) (bFromSweep :type Boolean) (SweepResult :type "HitResult Structure (by ref)"))
  ; Boar vs Player Collision Logic
  (if (not (`self.IsDead`))
    (if (== (`GameplayStatics.GetObjectClass` OtherActor) "/Game/Blueprints/BP_Character.BP_Character_C")
      (`/Engine/EditorBlueprintResources/StandardMacros.DoOnce` false :!label _label
        (:`Completed`
          (`GameplayStatics.ApplyDamage` OtherActor (`self.DamageAmount`) null self))))))

(event `self.CollisionSphere.OnComponentEndOverlap`
  (params (OverlappedComponent :type "PrimitiveComponent Object Reference") (OtherActor :type "Actor Object Reference") (OtherComp :type "PrimitiveComponent Object Reference") (OtherBodyIndex :type Integer))
  ; Boar vs Player Collision Logic
  (if (not (`self.IsDead`))
    (if (== (`GameplayStatics.GetObjectClass` OtherActor) "/Game/Blueprints/BP_Character.BP_Character_C")
      (goto _label :!via `Reset`))))

(event `self.LedgeDetector.OnComponentEndOverlap`
  (params (OverlappedComponent :type "PrimitiveComponent Object Reference") (OtherActor :type "Actor Object Reference") (OtherComp :type "PrimitiveComponent Object Reference") (OtherBodyIndex :type Integer))
  ; Ledge Detection
  (`self.ChangeDirections`))

(event `self.WallDetector.OnComponentBeginOverlap`
  (params (OverlappedComponent :type "PrimitiveComponent Object Reference") (OtherActor :type "Actor Object Reference") (OtherComp :type "PrimitiveComponent Object Reference") (OtherBodyIndex :type Integer) (bFromSweep :type Boolean) (SweepResult :type "HitResult Structure (by ref)"))
  ; Wall Detection
  (`self.ChangeDirections`))

(event `self.EnemeyDetector.OnComponentBeginOverlap`
  (params (OverlappedComponent :type "PrimitiveComponent Object Reference") (OtherActor :type "Actor Object Reference") (OtherComp :type "PrimitiveComponent Object Reference") (OtherBodyIndex :type Integer) (bFromSweep :type Boolean) (SweepResult :type "HitResult Structure (by ref)"))
  ; BP_Enemy Detection
  (for _array_element (`PrimitiveComponent.GetOverlappingActors` (`self.EnemeyDetector`) "/Game/Blueprints/BP_Enemy.BP_Enemy_C")
    (if (!= _array_element self)
      (`self.ChangeDirections`))))

(event `self.ReceiveTick`
  (params (DeltaSeconds :type "Float (single-precision)"))
  ; Call these functions/events on every tick
  (`self.IsPlayerInAttackRange?`)
  (`self.UpdateAnimation`))

(event `IsPlayerInAttackRange?`
  (bind _sprite (`self.Sprite`))
  ; Is Player in range of boar attack?
  ;; Check boar is not dead
  (if (not (`self.IsDead`))
    ;; If player IS in range of boar's attack range
    (for _array_element (`PrimitiveComponent.GetOverlappingActors` (`self.AttackRange`) "/Game/Blueprints/BP_Character.BP_Character_C")
      (if (`PrimitiveComponent.IsOverlappingActor` (`self.AttackRange`) _array_element)
        ;; First check if boar is not currently receiving damage
        (if (not (`self.IsReceivingDamage`))
          ;; If it is NOT, allow the boar to attack
          (set `self.IsAttacking` true)
          (else
            ;; If it is, we overwrite the attack animation with boar getting hit
            (`PaperFlipbookComponent.SetFlipbook` _sprite "/Game/Assets/Mobs/Boar/Flipbooks/FB_Boar_Hit.FB_Boar_Hit")
            (`PaperFlipbookComponent.SetLooping` _sprite false)))))))

(event `self.AttackRange.OnComponentBeginOverlap`
  (params (OverlappedComponent :type "PrimitiveComponent Object Reference") (OtherActor :type "Actor Object Reference") (OtherComp :type "PrimitiveComponent Object Reference") (OtherBodyIndex :type Integer) (bFromSweep :type Boolean) (SweepResult :type "HitResult Structure (by ref)"))
  ; On player entering/leaving boar's attack range
  (if (== (`GameplayStatics.GetObjectClass` OtherActor) "/Game/Blueprints/BP_Character.BP_Character_C")
    (set `self.IsAttacking` true)))

(event `self.AttackRange.OnComponentEndOverlap`
  (params (OverlappedComponent :type "PrimitiveComponent Object Reference") (OtherActor :type "Actor Object Reference") (OtherComp :type "PrimitiveComponent Object Reference") (OtherBodyIndex :type Integer))
  ; On player entering/leaving boar's attack range
  (if (== (`GameplayStatics.GetObjectClass` OtherActor) "/Game/Blueprints/BP_Character.BP_Character_C")
    (set `self.IsAttacking` false)))

(fn `ChangeDirections`
  (`self.K2_SetActorRotation` (`KismetMathLibrary.ComposeRotators` (`self.K2_GetActorRotation`) (struct :`Yaw` 180.0))))

(fn `EndHitstop`
  (set `self.CustomTimeDilation` 1.0))

(fn `EndSpriteFlickerEffect`
  (`KismetSystemLibrary.K2_ClearAndInvalidateTimerHandle` (`self.SpriteFlickerEffectRef`))
  (`SceneComponent.SetVisibility` (`self.Sprite`) true false))

(fn `StartHitstop`
  (params (Duration :type "Float (single-precision)"))
  (set `self.CustomTimeDilation` 0.0)
  (`KismetSystemLibrary.K2_SetTimer` null "EndHitstop" Duration))

(fn `StartSpriteFlickerEffect`
  (bind _returnvalue (`KismetSystemLibrary.K2_SetTimerDelegate` (`|CreateDelegate` :!event `ToggleSpriteFlickerEffect`) (`self.FlickerInterval`) true))
  (set `self.SpriteFlickerEffectRef` _returnvalue))

(fn `ToggleSpriteFlickerEffect`
  (bind _sprite (`self.Sprite`))
  (`SceneComponent.SetVisibility` _sprite (not (`SceneComponent.bVisible` _sprite)) false))

(fn `UpdateAnimation`
  (bind _sprite (`self.Sprite`))
  ; Only set movement-related animation if boar is NOT receiving damage
  (if (not (`self.IsReceivingDamage`))
    ; If boar is attacking, increase the max movement speed (walk speed), set flipbook and call play in case. If it is NOT, decrease the max movement speed (walk speed).
    (if (`self.IsAttacking`)
      (set `CharacterMovementComponent.MaxWalkSpeed` 120.0 (`self.CharacterMovement`))
      (`PaperFlipbookComponent.SetFlipbook` _sprite "/Game/Assets/Mobs/Boar/Flipbooks/FB_Boar_Run.FB_Boar_Run")
      (else
        (set `CharacterMovementComponent.MaxWalkSpeed` 60.0 (`self.CharacterMovement`))
        (`PaperFlipbookComponent.SetFlipbook` _sprite "/Game/Assets/Mobs/Boar/Flipbooks/FB_Boar_Walk.FB_Boar_Walk")))
    (`PaperFlipbookComponent.Play` (`self.Sprite`))))

(fn `UserConstructionScript`)