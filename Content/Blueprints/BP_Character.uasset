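; Player character for a 2D Paper2D side-scroller, handling movement, jumping, sword attacks, health, gem pickups and game-over, win and pause states.
; Tick selects flipbooks from movement and state, and uses animation frames to time footsteps and hitbox damage with brief hitstop.
; Damage triggers material flash, knockback and temporary input lockout.
; BeginPlay creates the HUD and parallax materials; interface events let other Blueprints update gems, health and death.
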(event `self.ReceiveBeginPlay`
  (bind _returnvalue (`GameplayStatics.GetPlayerController` 0))
  ; Initialize variables and setup
  ;; Enable player control with our Input Mapping Control (IMC)
  (`EnhancedInputSubsystemInterface.AddMappingContext` (pcsubsystem `EnhancedInputLocalPlayerSubsystem` _returnvalue) "/Game/Inputs/IMC_2DGameMapping.IMC_2DGameMapping" 0 (struct))
  (`WidgetBlueprintLibrary.SetInputMode_GameOnly` _returnvalue)
  ;; Create a dynamic sprite material instance reference to be used with trigger flash effect
  (bind _returnvalue_2 (`PrimitiveComponent.CreateDynamicMaterialInstance` (`self.Sprite`) 0 null "None"))
  (set `self.DynamicSpriteMat_FlashEffect` _returnvalue_2)
  ;; Create our In Game HUD
  (bind _returnvalue_3 (`|CreateWidget` "/Game/Widget/WBP_InGame.WBP_InGame_C" (`GameplayStatics.GetPlayerController` 0)))
  (bind _output_get (set `self.InGameHUD Ref` _returnvalue_3))
  (`UserWidget.AddToViewport` _output_get 0)
  (bind _output_get_2 (set `self.Health` 3.0))
  (`/Game/Widget/WBP_InGame.SetHealthIconBrush` (`self.InGameHUD Ref`) _output_get_2)
  ; Create and save references to dynamic material instances in an array for the parallax layers
  (for (_array_element _array_index) (`SceneComponent.GetChildrenComponents` (`self.StaticBackground`) false)
    (bind _aspaper_sprite_component (cast `PaperSpriteComponent` _array_element))
    (bind _returnvalue_4 (`PrimitiveComponent.CreateDynamicMaterialInstance` _aspaper_sprite_component 0 null "None"))
    (`MaterialInstanceDynamic.SetScalarParameterValue` _returnvalue_4 "ParallaxMultiplier" (`|GetArrayItem` (`self.ParallaxMultipliers`) _array_index))
    (`/Game/Widget/WBP_InGame.SetTotalGems` (`self.InGameHUD Ref`) 0)))

(event `TriggerSpriteFlashEffect`
  (params (FlashMultiplier :type "Float (single-precision)" :default 1.0) (FlashColor :type "LinearColor Structure" :default (struct :`R` 1.0 :`A` 1.0)) (PlayRate :type "Float (single-precision)" :default 5.0))
  ; Trigger Sprite Flash Effect
  ;; Set the params of the dynamic sprite material instance to the event's input params
  (`MaterialInstanceDynamic.SetScalarParameterValue` (`self.DynamicSpriteMat_FlashEffect`) "FlashMultiplier" FlashMultiplier)
  (`MaterialInstanceDynamic.SetVectorParameterValue` (`self.DynamicSpriteMat_FlashEffect`) "FlashColor" FlashColor)
  ;; Set the play rate for the timeline of our Fade Out Effect and use the alpha value to smooth lerp the FlashMultiplier value
  (`TimelineComponent.SetPlayRate` (`self.FadeOutEffect`) PlayRate)
  (bind (_direction _alpha) (`Timeline|FadeOutEffect` :!via `PlayFromStart`)
    (:`Update`
      (`MaterialInstanceDynamic.SetScalarParameterValue` (`self.DynamicSpriteMat_FlashEffect`) "FlashMultiplier" (`KismetMathLibrary.Lerp` 0.0 FlashMultiplier _alpha)))))

(event `self.ReceiveTick`
  (params (DeltaSeconds :type "Float (single-precision)"))
  ; Call these functions/events on every tick
  (`self.UpdateAnimation`)
  (`self.Play_Footstep_Sound`)
  (`self.Check_Attack_Hitbox`))

(event `Check_Attack_Hitbox`
  (bind _returnvalue (`PaperFlipbookComponent.GetPlaybackPositionInFrames` (`self.Sprite`)))
  ; Check Attack Hitbox
  ;; Check if player sprite is playing attack animation
  (if (== (`PaperFlipbookComponent.GetFlipbook` (`self.Sprite`)) "/Game/Assets/Character/Flipbooks/FB_Character_Attack.FB_Character_Attack")
    ;; Check specific frames of attack animation
    (if (or (== _returnvalue 1) (== _returnvalue 5))
      ;; If attack frame connects, call hitcheck to apply damage and activate particle effect. Else, reset the do once nodes and ValidHit bool
      (`|ExecutionSequence`
        (:`then_0`
          (`/Engine/EditorBlueprintResources/StandardMacros.DoOnce` false :!label _label
            (:`Completed`
              (`self.HitCheck`)
              ;; Replace sound with sword swing file
              (`GameplayStatics.PlaySound2D` "/Game/Sounds/human_attack_miss.human_attack_miss" 0.3 1.0 0.0 null null))))
        (:`then_1`
          (if (`self.ValidHit`)
            (`/Engine/EditorBlueprintResources/StandardMacros.DoOnce` false :!label _label_2
              (:`Completed`
                (`ActorComponent.Activate` (`self.PA_Burst`) true)
                ;; Replace sound with hit sound file
                (`GameplayStatics.PlaySound2D` "/Game/Sounds/human_attack_hit.human_attack_hit" 0.3 1.0 0.0 null null))))))
      (else
        (`|ExecutionSequence`
          (:`then_0`
            (goto _label :!via `Reset`))
          (:`then_1`
            (goto _label_2 :!via `Reset`))
          (:`then_2`
            (set `self.ValidHit` false)))))))

(event `EnhancedInput|/Game/Inputs/Actions/IA_Move`
  (params (ActionValue :type "Float (double-precision)") (ElapsedSeconds :type "Float (double-precision)") (TriggeredSeconds :type "Float (double-precision)") (InputAction :type "InputAction Object Reference" :default "/Game/Inputs/Actions/IA_Move.IA_Move"))
  ; Enhanced Input Action for movement
  (:`Triggered`
    ;; Only allow movement when player is NOT attacking
    (if (not (`self.IsAttacking`))
      (`self.AddMovementInput` (1.0 0.0 0.0) ActionValue)
      ;; Rotate the player controller depending on which direction the player is moving
      (`Controller.SetControlRotation` (`self.GetController`) (select `bool` (> ActionValue 0.0) :`false` (`KismetMathLibrary.MakeRotator` 0.0 0.0 180.0) :`true` (`KismetMathLibrary.MakeRotator` 0.0))))))

(event `EnhancedInput|/Game/Inputs/Actions/IA_Jump`
  (params (ActionValue :type Boolean) (ElapsedSeconds :type "Float (double-precision)") (TriggeredSeconds :type "Float (double-precision)") (InputAction :type "InputAction Object Reference" :default "/Game/Inputs/Actions/IA_Jump.IA_Jump"))
  ; Enhanced Input Action for jumping
  (:`Started`
    (`self.Jump`)
    (`GameplayStatics.PlaySound2D` "/Game/Sounds/jump.jump" 0.4 1.0 0.0 null null))
  (:`Completed`
    (`self.StopJumping`)))

(event `EnhancedInput|/Game/Inputs/Actions/IA_Attack`
  (params (ActionValue :type Boolean) (ElapsedSeconds :type "Float (double-precision)") (TriggeredSeconds :type "Float (double-precision)") (InputAction :type "InputAction Object Reference" :default "/Game/Inputs/Actions/IA_Attack.IA_Attack"))
  (bind _sprite (`self.Sprite`))
  ; Enhanced Input Action for attacking
  (:`Started`
    ;; Set IsAttacking bool, flipbook, and looping
    (set `self.IsAttacking` true)
    (`PaperFlipbookComponent.SetLooping` _sprite false)
    (`PaperFlipbookComponent.SetFlipbook` _sprite "/Game/Assets/Character/Flipbooks/FB_Character_Attack.FB_Character_Attack")))

(event `self.Sprite.OnFinishedPlaying`
  (bind _sprite (`self.Sprite`))
  ; On Sprite finishes playing
  (if (not (`self.IsDead`))
    ;; When attack animation finishes playing, set IsAttacking bool, looping, and call play on current flipbook animation (ie - idle, run)
    (set `self.IsAttacking` false)
    (`PaperFlipbookComponent.SetLooping` _sprite true)
    (`PaperFlipbookComponent.Play` _sprite)
    (else
      (`self.SetGameOver`))))

(event `SetGameOver`
  (bind _returnvalue (`GameplayStatics.GetPlayerController` 0))
  (bind _ingamehud_ref (`self.InGameHUD Ref`))
  (bind _menutext (`/Game/Widget/WBP_InGame.MenuText` _ingamehud_ref))
  (bind _quitbutton (`/Game/Widget/WBP_InGame.QuitButton` _ingamehud_ref))
  (bind _returnmenubutton (`/Game/Widget/WBP_InGame.ReturnMenuButton` _ingamehud_ref))
  ; set GAME OVER text to visible in HUD, "freeze" game, and allows mouse cursor input
  (`TextBlock.SetText` _menutext "Game Over")
  (`Widget.SetVisibility` _menutext "Visible")
  (`GameplayStatics.SetGamePaused` true)
  (`Widget.SetVisibility` _quitbutton "Visible")
  (`Widget.SetIsEnabled` _quitbutton true)
  (`Widget.SetVisibility` _returnmenubutton "Visible")
  (`Widget.SetIsEnabled` _returnmenubutton true)
  (set `PlayerController.bShowMouseCursor` true _returnvalue)
  (`WidgetBlueprintLibrary.SetInputMode_UIOnlyEx` _returnvalue null))

(event `Play_Footstep_Sound`
  (bind _sprite (`self.Sprite`))
  (bind _returnvalue (`PaperFlipbookComponent.GetPlaybackPositionInFrames` _sprite))
  ; Footstep Sound Logic
  ;; Check if player sprite is playing run animation
  (if (== (`PaperFlipbookComponent.GetFlipbook` _sprite) "/Game/Assets/Character/Flipbooks/FB_Character_Run.FB_Character_Run")
    ;; Check specific frames of run animation
    (if (or (== _returnvalue 3) (== _returnvalue 7))
      (`/Engine/EditorBlueprintResources/StandardMacros.DoOnce` false :!label _label_3
        (:`Completed`
          ;; Replace sound with footstep sound file
          (`GameplayStatics.PlaySoundAtLocation` "/Game/Sounds/footsteps.footsteps" (`self.K2_GetActorLocation`) (struct) 0.1 1.0 0.0 null null null null)))
      (else
        (goto _label_3 :!via `Reset`)))))

(event `self.ReceiveAnyDamage`
  (params (Damage :type "Float (single-precision)") (DamageType :type "DamageType Object Reference") (InstigatedBy :type "Controller Object Reference") (DamageCauser :type "Actor Object Reference"))
  ; On incoming damage
  (if (> Damage 0.0)
    ;; Check if player is not already receiving damage
    (if (not (`self.IsReceivingDamage`))
      ;; Temporarily disable player input when receiving damage
      (set `self.IsReceivingDamage` true)
      (`self.DisableInput` (`GameplayStatics.GetPlayerController` 0))
      ;; Trigger sprite flash effect
      (`self.TriggerSpriteFlashEffect` 1.0 (struct :`R` 1.0 :`A` 1.0) 0.8)
      (`self.UpdateHealth` Damage)
      ;; Replace sound with hit sound file
      (`GameplayStatics.PlaySound2D` "/Game/Sounds/damage1.damage1" 0.2 1.0 0.0 null null)
      (`self.KnockbackEffect` DamageCauser)
      (`KismetSystemLibrary.Delay` 0.5)
      (if (<= (`self.Health`) 0.0)
        (set `self.IsDead` true)
        (`GameplayStatics.PlaySound2D` "/Game/Sounds/human_death.human_death" 0.3 1.0 0.0 null null)
        (else
          ;; If player is not dead, re-enable input
          (set `self.IsReceivingDamage` false)
          (`self.EnableInput` (`GameplayStatics.GetPlayerController` 0)))))
    (else
      (`self.TriggerSpriteFlashEffect` 1.0 (struct :`G` 1.0 :`A` 1.0) 0.8)
      (`self.UpdateHealth` Damage)
      (`GameplayStatics.PlaySound2D` "/Game/Sounds/damage1.damage1" 0.2 1.0 0.0 null null))))

(event `/Game/Blueprints/Interfaces/BPI_Character.UpdateGemCount`
  ; BP_Character implements the BPI_Character interface. This allows us to hook up the UpdateGemCount event from the BPI_Character interface to logic in BP_Character and we can call this event in another blueprint (w/o the need to cast)
  (bind _result (`/Engine/EditorBlueprintResources/StandardMacros.IncrementInt` (`self.numGemsCollected`))
    (:`  `
      (bind _output_get (set `self.numGemsCollected` _result))
      (`/Game/Widget/WBP_InGame.SetTotalGems` (`self.InGameHUD Ref`) _output_get)
      (`GameplayStatics.PlaySound2D` "/Game/Sounds/coin.coin" 0.3 1.0 0.0 null null))))

(event `/Game/Blueprints/Interfaces/BPI_Character.IncrementHealth`
  (params (Damage :type "Float (double-precision)"))
  ; BP Interface event to increment player health
  (`self.TriggerSpriteFlashEffect` 1.0 (struct :`G` 1.0 :`A` 1.0) 0.8)
  (`self.UpdateHealth` Damage)
  (`GameplayStatics.PlaySound2D` "/Game/Sounds/power_up.power_up" 0.3 1.0 0.0 null null))

(event `/Game/Blueprints/Interfaces/BPI_Character.DecrementHealth`
  (params (DamageAmount :type "Float (double-precision)"))
  (`self.TriggerSpriteFlashEffect` 1.0 (struct :`R` 1.0 :`A` 1.0) 0.8)
  (`self.UpdateHealth` DamageAmount))

(event `/Game/Blueprints/Interfaces/BPI_PawnActor.SetIsDead`
  ; BP Interface event to set character's IsDead to true and play sound
  (set `self.IsDead` true)
  (`GameplayStatics.PlaySound2D` "/Game/Sounds/human_death.human_death" 0.3 1.0 0.0 null null))

(event `Key|P` :paused true
  (params (Key :type "Key Structure"))
  ; Allows player to pause/unpause game
  (:`Pressed`
    (if (not (`self.IsDead`))
      (`self.TogglePauseMenu`))))

(event `TogglePauseMenu`
  (bind _menutext (`/Game/Widget/WBP_InGame.MenuText` (`self.InGameHUD Ref`)))
  ; Allows player to pause/unpause game
  (if (not (`GameplayStatics.IsGamePaused`))
    (`TextBlock.SetText` _menutext "Game Paused")
    (`Widget.SetVisibility` _menutext "Visible")
    (`GameplayStatics.SetGamePaused` true)
    (else
      (`Widget.SetVisibility` (`/Game/Widget/WBP_InGame.MenuText` (`self.InGameHUD Ref`)) "Hidden")
      (`GameplayStatics.SetGamePaused` false))))

(event `/Game/Blueprints/Interfaces/BPI_Character.DisplayWin`
  (bind _returnvalue (`GameplayStatics.GetPlayerController` 0))
  (bind _ingamehud_ref (`self.InGameHUD Ref`))
  (bind _menutext (`/Game/Widget/WBP_InGame.MenuText` _ingamehud_ref))
  (bind _returnmenubutton (`/Game/Widget/WBP_InGame.ReturnMenuButton` _ingamehud_ref))
  (bind _quitbutton (`/Game/Widget/WBP_InGame.QuitButton` _ingamehud_ref))
  (`TextBlock.SetText` _menutext "Congrats! You made it home!")
  (`Widget.SetVisibility` _menutext "Visible")
  (`GameplayStatics.SetGamePaused` true)
  (`Widget.SetVisibility` _quitbutton "Visible")
  (`Widget.SetIsEnabled` _quitbutton true)
  (`Widget.SetVisibility` _returnmenubutton "Visible")
  (`Widget.SetIsEnabled` _returnmenubutton true)
  (set `PlayerController.bShowMouseCursor` true _returnvalue)
  (`WidgetBlueprintLibrary.SetInputMode_UIOnlyEx` _returnvalue null))

(fn `EndHitstop`
  (set `self.CustomTimeDilation` 1.0))

(fn `HitCheck`
  ; Checks if hitbox overlaps with BP_Enemy and apply damage to them
  (for _array_element (`PrimitiveComponent.GetOverlappingActors` (`self.Hitbox`) "/Game/Blueprints/BP_Enemy.BP_Enemy_C")
    (`GameplayStatics.ApplyDamage` _array_element (`self.DamageAmount`))
    (set `self.ValidHit` true)
    (`self.StartHitstop` 0.05)))

(fn `KnockbackEffect`
  (params (DamageCauser :type "Actor Object Reference"))
  (bind _returnvalue_x (`KismetMathLibrary.BreakVector` (`self.K2_GetActorLocation` DamageCauser)))
  (bind _returnvalue_x_2 (`KismetMathLibrary.BreakVector` (`self.K2_GetActorLocation`)))
  ; Launch player back in opposite direction from the damage causer to simulate knockback effect
  (set `MovementComponent.Velocity` (0.0 0.0 0.0) (`self.CharacterMovement`))
  (if (>= _returnvalue_x _returnvalue_x_2)
    (`self.LaunchCharacter` (-300.0 0.0 500.0))
    (else
      (`self.LaunchCharacter` (300.0 0.0 500.0)))))

(fn `StartHitstop`
  (params (Duration :type "Float (single-precision)"))
  (set `self.CustomTimeDilation` 0.0)
  (`KismetSystemLibrary.K2_SetTimer` null "EndHitstop" Duration))

(fn `UpdateAnimation`
  (bind (_returnvalue_x _returnvalue_y _returnvalue_z) (`KismetMathLibrary.BreakVector` (`self.GetVelocity`)))
  (bind _sprite (`self.Sprite`))
  (bind _sprite_2 (`self.Sprite`))
  (bind _sprite_3 (`self.Sprite`))
  ; Check if player is grounded
  (if (`NavMovementInterface.IsMovingOnGround` (`self.CharacterMovement`))
    ; Check if player is dead
    (if (not (`self.IsDead`))
      ; Check if player is NOT currently attacking
      (if (not (`self.IsAttacking`))
        ; Depending on player current velocity, play either the idle or run animation
        (if (> (`KismetMathLibrary.Abs` (`KismetMathLibrary.VSize` (`self.GetVelocity`))) 0.0)
          (`PaperFlipbookComponent.SetFlipbook` _sprite "/Game/Assets/Character/Flipbooks/FB_Character_Run.FB_Character_Run")
          (else
            (`PaperFlipbookComponent.SetFlipbook` _sprite "/Game/Assets/Character/Flipbooks/FB_Character_Idle.FB_Character_Idle"))))
      (else
        ; If so, set flipbook to death animation
        (`PaperFlipbookComponent.SetFlipbook` _sprite_3 "/Game/Assets/Character/Flipbooks/FB_Character_Dead.FB_Character_Dead")
        (`PaperFlipbookComponent.SetLooping` _sprite_3 false)))
    (else
      ; If not, player must be either jumping or falling. Set proper flipbook depending on current Z velocity
      (if (< _returnvalue_z -100.0)
        (`PaperFlipbookComponent.SetFlipbook` _sprite_2 "/Game/Assets/Character/Flipbooks/FB_Character_Fall.FB_Character_Fall")
        (else
          (`PaperFlipbookComponent.SetFlipbook` _sprite_2 "/Game/Assets/Character/Flipbooks/FB_Character_Jump.FB_Character_Jump"))))))

(fn `UpdateHealth`
  (params (Damage :type "Float (double-precision)"))
  (bind _returnvalue (- (`self.Health`) Damage))
  ; Update player health and HUD
  (if (<= _returnvalue 0.0)
    (bind _output_get (set `self.Health` 0.0))
    (`/Game/Widget/WBP_InGame.SetHealthIconBrush` (`self.InGameHUD Ref`) _output_get)
    (`self.DisableInput` (`GameplayStatics.GetPlayerController` 0))
    (else
      (if (>= _returnvalue 3.0)
        (set `self.Health` 3.0)
        (else
          (set `self.Health` _returnvalue)))
      (`/Game/Widget/WBP_InGame.SetHealthIconBrush` (`self.InGameHUD Ref`) (`self.Health`)))))

(fn `UserConstructionScript`)