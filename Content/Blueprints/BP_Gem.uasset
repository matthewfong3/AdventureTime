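; BP_Gem is a collectible gem pickup that the player character picks up by touching it.
; When its collision sphere overlaps an actor whose class is exactly BP_Character, it tells that character to update its gem count message.
; It then disables the sphere's collision, activates the PAItemFeedback component, hides the render component, and destroys itself after a short delay.
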(event `self.CollisionSphere.OnComponentBeginOverlap`
  (params (OverlappedComponent :type "PrimitiveComponent Object Reference") (OtherActor :type "Actor Object Reference") (OtherComp :type "PrimitiveComponent Object Reference") (OtherBodyIndex :type Integer) (bFromSweep :type Boolean) (SweepResult :type "HitResult Structure (by ref)"))
  (if (== (`GameplayStatics.GetObjectClass` OtherActor) "/Game/Blueprints/BP_Character.BP_Character_C")
    (message `/Game/Blueprints/Interfaces/BPI_Character.UpdateGemCount` OtherActor)
    (`PrimitiveComponent.SetCollisionEnabled` (`self.CollisionSphere`) "NoCollision")
    (`ActorComponent.Activate` (`self.PA_Item_Feedback`) false)
    (`SceneComponent.SetVisibility` (`self.RenderComponent`) false false)
    (`KismetSystemLibrary.Delay` 1.0)
    (`self.K2_DestroyActor`)))

(fn `UserConstructionScript`)