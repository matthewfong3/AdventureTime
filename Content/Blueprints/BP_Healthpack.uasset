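; BP_Healthpack is a pickup that restores health when a BP_Character overlaps its collision sphere.
; It sends IncrementHealth with -1.0 through the BPI_Character interface; an equivalent negative ApplyDamage node is left unconnected.
; On pickup it disables collision, activates PAItemFeedback and hides the render component, then destroys itself after a short delay.
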(event `self.CollisionSphere.OnComponentBeginOverlap`
  (params (OverlappedComponent :type "PrimitiveComponent Object Reference") (OtherActor :type "Actor Object Reference") (OtherComp :type "PrimitiveComponent Object Reference") (OtherBodyIndex :type Integer) (bFromSweep :type Boolean) (SweepResult :type "HitResult Structure (by ref)"))
  ; We can use either methods to add health. We can apply negative damage which will be taken care of in BP_Character's UpdateHealth function. Or we can call IncrementHealth event since BP_Character implements BPI_Character interface
  (if (== (`GameplayStatics.GetObjectClass` OtherActor) "/Game/Blueprints/BP_Character.BP_Character_C")
    (message `/Game/Blueprints/Interfaces/BPI_Character.IncrementHealth` OtherActor -1.0)
    (`PrimitiveComponent.SetCollisionEnabled` (`self.CollisionSphere`) "NoCollision")
    (`ActorComponent.Activate` (`self.PA_Item_Feedback`) false)
    (`SceneComponent.SetVisibility` (`self.RenderComponent`) false false)
    (`KismetSystemLibrary.Delay` 1.0)
    (`self.K2_DestroyActor`)))

(fn `UserConstructionScript`)