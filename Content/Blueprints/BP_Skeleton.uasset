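; BP_Skeleton is a 2D flipbook enemy that roams, seeks the player along X, and deals contact and melee damage.
; Move drives roaming or seeking, with detector components reversing direction at walls, ledges and other enemies.
; Tick checks the attack range, applying hits on a specific flipbook frame.
; Incoming damage interrupts attacks with a material flash and time-dilation hitstop, while death adds sprite flicker before destroying the actor.
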(event `self.ReceiveBeginPlay`
  ; Create a dynamic sprite material instance reference to be used with trigger flash effect. Initialize health
  (bind _returnvalue (`PrimitiveComponent.CreateDynamicMaterialInstance` (`self.Sprite`) 0 null "None"))
  (set `self.DynamicSpriteMaterialInstance` _returnvalue)
  (set `self.Health` 300.0))

(event `TriggerSpriteFlashEffect`
  (params (FlashMultiplier :type "Float (single-precision)" :default 1.0) (FlashColor :type "LinearColor Structure" :default (struct :`R` 1.0 :`A` 1.0)) (PlayRate :type "Float (single-precision)" :default 5.0))
  ; Trigger Sprite Flash Effect
  ;; Set the dynamic sprite material instance params to the event's input params
  (`MaterialInstanceDynamic.SetScalarParameterValue` (`self.DynamicSpriteMaterialInstance`) "FlashMultiplier" FlashMultiplier)
  (`MaterialInstanceDynamic.SetVectorParameterValue` (`self.DynamicSpriteMaterialInstance`) "FlashColor" FlashColor)
  ;; Set the play rate for the timeline of our Fade Out Effect and use the alpha value to smooth lerp the FlashMultiplier value
  (`TimelineComponent.SetPlayRate` (`self.FadeOutEffect`) PlayRate)
  (bind (_direction _alpha) (`Timeline|FadeOutEffect` :!via `PlayFromStart`)
    (:`Update`
      (`MaterialInstanceDynamic.SetScalarParameterValue` (`self.DynamicSpriteMaterialInstance`) "FlashMultiplier" (`KismetMathLibrary.Lerp` 0.0 FlashMultiplier _alpha)))))

(event `self.ReceiveTick`
  (params (DeltaSeconds :type "Float (single-precision)"))
  ; Call these functions/events on every tick
  (`self.IsPlayerInAttackRange?`))

(event `Move`
  ; Allows Skeleton to move (seek player or roam freely)
  (if (`self.IsSeeking`)
    (`self.Seek`)
    (else
      ;; "Free Roam"
      (`self.AddMovementInput` (`self.GetActorForwardVector`)))))

(event `self.WallDetector.OnComponentBeginOverlap`
  (params (OverlappedComponent :type "PrimitiveComponent Object Reference") (OtherActor :type "Actor Object Reference") (OtherComp :type "PrimitiveComponent Object Reference") (OtherBodyIndex :type Integer) (bFromSweep :type Boolean) (SweepResult :type "HitResult Structure (by ref)"))
  ; Wall Detection
  (`self.ChangeDirections`))

(event `self.EnemyDetector.OnComponentBeginOverlap`
  (params (OverlappedComponent :type "PrimitiveComponent Object Reference") (OtherActor :type "Actor Object Reference") (OtherComp :type "PrimitiveComponent Object Reference") (OtherBodyIndex :type Integer) (bFromSweep :type Boolean) (SweepResult :type "HitResult Structure (by ref)"))
  ; BP_Enemy Detection
  (if (not (`self.IsSeeking`))
    (for _array_element (`PrimitiveComponent.GetOverlappingActors` (`self.EnemyDetector`) "/Game/Blueprints/BP_Enemy.BP_Enemy_C")
      (if (!= _array_element self)
        (`self.ChangeDirections`)))))

(event `self.LedgeDetector.OnComponentEndOverlap`
  (params (OverlappedComponent :type "PrimitiveComponent Object Reference") (OtherActor :type "Actor Object Reference") (OtherComp :type "PrimitiveComponent Object Reference") (OtherBodyIndex :type Integer))
  ; Ledge Detection
  (`self.ChangeDirections`))

(event `self.ReceiveAnyDamage`
  (params (Damage :type "Float (single-precision)") (DamageType :type "DamageType Object Reference") (InstigatedBy :type "Controller Object Reference") (DamageCauser :type "Actor Object Reference"))
  (bind _sprite (`self.Sprite`))
  ; Apply incoming damage
  ;; Overwrite IsAttacking state when receiving damage
  (set `self.IsAttacking` false)
  ;; Trigger sprite flash effect and apply hitstop effect
  (`self.TriggerSpriteFlashEffect` 1.0 (struct :`R` 1.0 :`A` 1.0) 3.0)
  (`self.StartHitstop` 0.05)
  (`GameplayStatics.PlaySound2D` "/Game/Sounds/damage1.damage1" 0.15 1.0 0.0 null null)
  (set `self.Health` (- (`self.Health`) Damage))
  (set `self.IsReceivingDamage` true)
  (if (<= (`self.Health`) 0.0)
    ;; Skeleton == dead, set flipbook, looping, play the sprite flicker effect upon death, disable capsule collision component. After small delay, destroy actor
    (set `self.IsDead` true)
    (`PaperFlipbookComponent.SetFlipbook` _sprite "/Game/Assets/Mobs/Skeleton/Flipbooks/FB_Skeleton_Dead.FB_Skeleton_Dead")
    (`PaperFlipbookComponent.SetLooping` (`self.Sprite`) false)
    (`self.StartSpriteFlickerEffect`)
    (`PrimitiveComponent.SetCollisionEnabled` (`self.CapsuleComponent`) "NoCollision")
    (`GameplayStatics.PlaySound2D` "/Game/Sounds/enemy_death.enemy_death" 1.0 1.0 0.0 null null)
    (`KismetSystemLibrary.Delay` 1.5)
    (`self.K2_DestroyActor`)
    (else
      ;; Skeleton != dead, set flipbook, looping
      (`PaperFlipbookComponent.SetFlipbook` _sprite "/Game/Assets/Mobs/Skeleton/Flipbooks/FB_Skeleton_Hit.FB_Skeleton_Hit")
      (`PaperFlipbookComponent.SetLooping` (`self.Sprite`) false))))

(event `self.Sprite.OnFinishedPlaying`
  (bind _sprite (`self.Sprite`))
  ; On Sprite finish playing
  ;; Check Skeleton != dead
  (if (not (`self.IsDead`))
    ;; After hit || attack animation finishes playing, Skeleton is no longer receiving damage || attacking, reset flipbook animation to walk, reset looping to true and call Play node on sprite component
    (if (`self.IsReceivingDamage`)
      (set `self.IsReceivingDamage` false)
      (if (`self.ChangedForwardVectorOnSeek`) :!label _label
        (set `self.ChangedForwardVectorOnSeek` false)
        (`self.ChangeDirections`))
      (`PaperFlipbookComponent.SetFlipbook` _sprite "/Game/Assets/Mobs/Skeleton/Flipbooks/FB_Skeleton_Walk.FB_Skeleton_Walk")
      (`PaperFlipbookComponent.SetLooping` _sprite true)
      (`PaperFlipbookComponent.Play` _sprite)
      (elif (`self.IsAttacking`)
        (set `self.IsAttacking` false)
        (goto _label)))))

(event `self.Collisionbox.OnComponentBeginOverlap`
  (params (OverlappedComponent :type "PrimitiveComponent Object Reference") (OtherActor :type "Actor Object Reference") (OtherComp :type "PrimitiveComponent Object Reference") (OtherBodyIndex :type Integer) (bFromSweep :type Boolean) (SweepResult :type "HitResult Structure (by ref)"))
  ; Skeleton and Player Collision Logic
  ;; Check Skeleton != dead
  (if (not (`self.IsDead`))
    ;; If the actor that bumped into the Skeleton is our BP_Character, apply damage to our BP_Character
    (if (== (`GameplayStatics.GetObjectClass` OtherActor) "/Game/Blueprints/BP_Character.BP_Character_C")
      (`/Engine/EditorBlueprintResources/StandardMacros.DoOnce` false :!label _label_2
        (:`Completed`
          (`GameplayStatics.ApplyDamage` OtherActor (`self.DamageAmount`) null self))))))

(event `self.Collisionbox.OnComponentEndOverlap`
  (params (OverlappedComponent :type "PrimitiveComponent Object Reference") (OtherActor :type "Actor Object Reference") (OtherComp :type "PrimitiveComponent Object Reference") (OtherBodyIndex :type Integer))
  ; Skeleton and Player Collision Logic
  ;; Check Skeleton != dead
  (if (not (`self.IsDead`))
    ;; If the actor that bumped into the Skeleton is our BP_Character, apply damage to our BP_Character
    (if (== (`GameplayStatics.GetObjectClass` OtherActor) "/Game/Blueprints/BP_Character.BP_Character_C")
      (goto _label_2 :!via `Reset`))))

(event `IsPlayerInAttackRange?`
  (bind _sprite (`self.Sprite`))
  (bind _sprite_2 (`self.Sprite`))
  ; Is Player in range of Skeleton attack?
  ;; Check Skeleton != dead
  (if (not (`self.IsDead`))
    ;; Check if player IS in range of Skeleton attack range
    (for _array_element (`PrimitiveComponent.GetOverlappingActors` (`self.HitboxRange`) "/Game/Blueprints/BP_Character.BP_Character_C")
      (if (`PrimitiveComponent.IsOverlappingActor` (`self.HitboxRange`) _array_element)
        ;; First check that skeleton != receiving damage
        (if (not (`self.IsReceivingDamage`))
          ;; If it is NOT receiving damage, allow the skeleton to attack. Then call Check_Attack_Hitbox to see if attack connected
          (set `self.IsAttacking` true)
          (`PaperFlipbookComponent.SetFlipbook` _sprite "/Game/Assets/Mobs/Skeleton/Flipbooks/FB_Skeleton_Attack.FB_Skeleton_Attack")
          (`PaperFlipbookComponent.SetLooping` _sprite false)
          (`self.Check_Attack_Hitbox`)
          (else
            ;; If it is, we overwrite the attack animation with skeleton getting hit
            (`PaperFlipbookComponent.SetFlipbook` _sprite_2 "/Game/Assets/Mobs/Skeleton/Flipbooks/FB_Skeleton_Hit.FB_Skeleton_Hit")
            (`PaperFlipbookComponent.SetLooping` _sprite_2 false)))))))

(event `Check_Attack_Hitbox`
  ; Check Attack Hitbox
  ;; Check if skeleton is playing attack animation
  (if (== (`PaperFlipbookComponent.GetFlipbook` (`self.Sprite`)) "/Game/Assets/Mobs/Skeleton/Flipbooks/FB_Skeleton_Attack.FB_Skeleton_Attack")
    ;; If attack frame connects, call HitCheck to apply damage. Else, reset the do once node
    (if (== (`PaperFlipbookComponent.GetPlaybackPositionInFrames` (`self.Sprite`)) 7)
      (`/Engine/EditorBlueprintResources/StandardMacros.DoOnce` false :!label _label_3
        (:`Completed`
          (`GameplayStatics.PlaySound2D` "/Game/Sounds/skeleton_attack.skeleton_attack" 0.3 1.0 0.0 null null)
          (`self.HitCheck`)))
      (else
        (goto _label_3 :!via `Reset`)))))

(event `self.SeekRange.OnComponentBeginOverlap`
  (params (OverlappedComponent :type "PrimitiveComponent Object Reference") (OtherActor :type "Actor Object Reference") (OtherComp :type "PrimitiveComponent Object Reference") (OtherBodyIndex :type Integer) (bFromSweep :type Boolean) (SweepResult :type "HitResult Structure (by ref)"))
  ; On player entering/leaving the Skeleton's seek range
  (if (== (`GameplayStatics.GetObjectClass` OtherActor) "/Game/Blueprints/BP_Character.BP_Character_C")
    (`self.ActorToSeekRef`
      (:`then`
        _)
      (:`else`
        (set `self.ActorToSeekRef` OtherActor)))
    (set `self.IsSeeking` true)))

(event `self.SeekRange.OnComponentEndOverlap`
  (params (OverlappedComponent :type "PrimitiveComponent Object Reference") (OtherActor :type "Actor Object Reference") (OtherComp :type "PrimitiveComponent Object Reference") (OtherBodyIndex :type Integer))
  ; On player entering/leaving the Skeleton's seek range
  (if (== (`GameplayStatics.GetObjectClass` OtherActor) "/Game/Blueprints/BP_Character.BP_Character_C")
    (set `self.IsSeeking` false)
    (if (not (`self.IsAttacking`))
      (if (`self.ChangedForwardVectorOnSeek`)
        (set `self.ChangedForwardVectorOnSeek` false)
        (`self.ChangeDirections`)))))

(fn `ChangeDirections`
  (`self.K2_SetActorRotation` (`KismetMathLibrary.ComposeRotators` (`self.K2_GetActorRotation`) (struct :`Yaw` 180.0))))

(fn `EndHitstop`
  (set `self.CustomTimeDilation` 1.0))

(fn `EndSpriteFlickerEffect`
  ; With the flicker effect timer reference, clear and invalidate the timer and set sprite component visibility to true just in case
  (`KismetSystemLibrary.K2_ClearAndInvalidateTimerHandle` (`self.SpriteFlickerEffectTimer`))
  (`SceneComponent.SetVisibility` (`self.Sprite`) true false))

(fn `HitCheck`
  ; Checks if hitbox overlaps with BP_Character and apply damage to them
  (for _array_element (`PrimitiveComponent.GetOverlappingActors` (`self.HitboxRange`) "/Game/Blueprints/BP_Character.BP_Character_C")
    (`GameplayStatics.ApplyDamage` _array_element (`self.DamageAmount`) null self)))

(fn `Seek`
  (bind _returnvalue_x (`KismetMathLibrary.BreakVector` (`self.K2_GetActorLocation`)))
  (bind _returnvalue_x_2 (`KismetMathLibrary.BreakVector` (`self.K2_GetActorLocation`)))
  (bind _returnvalue_x_3 (`KismetMathLibrary.BreakVector` (`self.GetActorForwardVector`)))
  (bind _returnvalue_x_4 (`KismetMathLibrary.BreakVector` (`self.K2_GetActorLocation`)))
  (bind _returnvalue_x_5 (`KismetMathLibrary.BreakVector` (`self.K2_GetActorLocation` (`self.ActorToSeekRef`))))
  ; A simple AI seek implementation for when the player is in range of skeleton. Skeleton will start to seek the player's location
  (bind _actortoseekref (`self.ActorToSeekRef`)
    (:`then`
      (bind _returnvalue_x_6 (`KismetMathLibrary.BreakVector` (`self.K2_GetActorLocation` _actortoseekref)))
      (bind _output_get (set `self.DesiredSeekVector` (`KismetMathLibrary.Normal` (`KismetMathLibrary.MakeVector` (- _returnvalue_x_6 _returnvalue_x_2)) 0.0)))
      (if (!= (+ _returnvalue_x_4 (.x _output_get)) (+ _returnvalue_x_4 _returnvalue_x_3))
        (`self.ChangeDirections`)
        (set `self.ChangedForwardVectorOnSeek` true))
      (if (< _returnvalue_x_5 _returnvalue_x)
        _
        (else
          _))
      (`self.AddMovementInput` (`self.GetActorForwardVector`)))
    (:`else`)))

(fn `StartHitstop`
  (params (Duration :type "Float (double-precision)"))
  (set `self.CustomTimeDilation` 0.0)
  (`KismetSystemLibrary.K2_SetTimer` null "EndHitstop" Duration))

(fn `StartSpriteFlickerEffect`
  ; Create an event to call the ToggleSpriteFlickerEffect() by timer (every Flicker Interval)
  (bind _returnvalue (`KismetSystemLibrary.K2_SetTimerDelegate` (`|CreateDelegate` :!event `ToggleSpriteFlickerEffect`) (`self.FlickerInterval`) true))
  ; Save a reference to the return timer so we can stop the flicker effect
  (set `self.SpriteFlickerEffectTimer` _returnvalue))

(fn `ToggleSpriteFlickerEffect`
  (bind _sprite (`self.Sprite`))
  (`SceneComponent.SetVisibility` _sprite (not (`SceneComponent.bVisible` _sprite)) false))

(fn `UserConstructionScript`)