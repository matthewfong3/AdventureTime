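; Paper2D snail enemy that walks, turns around when its detector components report other enemies, walls or ledges, and damages BP_Character on contact.
; MoveForward supplies movement input, while a DoOnce reset on overlap end limits damage to one hit per contact.
; Taking damage triggers a timeline-faded red material flash, hitstop via CustomTimeDilation, sound and hit flipbook.
; At zero health it disables capsule collision, flickers on a timer, then destroys itself.
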(event `self.ReceiveBeginPlay`
  ; Create a dynamic material instance and save a reference to it for the Trigger Sprite Flash Effect. Initialize health
  (bind _returnvalue (`PrimitiveComponent.CreateDynamicMaterialInstance` (`self.Sprite`) 0 null "None"))
  (set `self.DynamicSpriteMaterialRef` _returnvalue)
  (set `self.Health` 150.0))

(event `TriggerSpriteFlashEffect`
  (params (FlashMultiplier :type "Float (single-precision)" :default 1.0) (FlashColor :type "LinearColor Structure" :default (struct :`R` 1.0 :`B` 0.026156 :`A` 1.0)) (PlayRate :type "Float (single-precision)" :default 5.0))
  ; Trigger Sprite Flash Effect
  ;; Set the params of the dynamic sprite material instance to the event's input params
  (`MaterialInstanceDynamic.SetScalarParameterValue` (`self.DynamicSpriteMaterialRef`) "FlashMultiplier" FlashMultiplier)
  (`MaterialInstanceDynamic.SetVectorParameterValue` (`self.DynamicSpriteMaterialRef`) "FlashColor" FlashColor)
  ;; Set the play rate for the timeline of our Fade Out Effect and use the alpha value to smooth lerp the FlashMultiplier value
  (`TimelineComponent.SetPlayRate` (`self.FadeOutEffect`) PlayRate)
  (bind (_direction _alpha) (`Timeline|FadeOutEffect` :!via `PlayFromStart`)
    (:`Update`
      (`MaterialInstanceDynamic.SetScalarParameterValue` (`self.DynamicSpriteMaterialRef`) "FlashMultiplier" (`KismetMathLibrary.Lerp` 0.0 FlashMultiplier _alpha)))))

(event `MoveForward`
  ; Allows Snail to move
  (`self.AddMovementInput` (`self.GetActorForwardVector`) -1.0))

(event `self.ReceiveAnyDamage`
  (params (Damage :type "Float (single-precision)") (DamageType :type "DamageType Object Reference") (InstigatedBy :type "Controller Object Reference") (DamageCauser :type "Actor Object Reference"))
  (bind _sprite (`self.Sprite`))
  ; Apply incoming damage
  ;; Trigger sprite flash effect and apply hitstop effect
  (`self.TriggerSpriteFlashEffect` 1.0 (struct :`R` 1.0 :`A` 1.0) 3.0)
  (`self.StartHitstop` 0.05)
  (`GameplayStatics.PlaySound2D` "/Game/Sounds/damage1.damage1" 0.15 1.0 0.0 null null)
  (set `self.Health` (- (`self.Health`) Damage))
  (set `self.IsReceivingDamage` true)
  (if (<= (`self.Health`) 0.0)
    ;; Snail == dead, set flipbook, looping, play the sprite flicker effect upon death, disable capsule collision component. After small delay, destroy actor
    (set `self.IsDead` true)
    (`PaperFlipbookComponent.SetFlipbook` _sprite "/Game/Assets/Mobs/Snail/Flipbooks/FB_Snail_Dead.FB_Snail_Dead")
    (`PaperFlipbookComponent.SetLooping` (`self.Sprite`) false)
    (`self.StartSpriteFlickerEffect`)
    (`PrimitiveComponent.SetCollisionEnabled` (`self.CapsuleComponent`) "NoCollision")
    (`GameplayStatics.PlaySound2D` "/Game/Sounds/enemy_death.enemy_death" 1.0 1.0 0.0 null null)
    (`KismetSystemLibrary.Delay` 1.0)
    (`self.K2_DestroyActor`)
    (else
      ;; Snail != dead, set flipbook, looping
      (`PaperFlipbookComponent.SetFlipbook` _sprite "/Game/Assets/Mobs/Snail/Flipbooks/FB_Snail_Hit.FB_Snail_Hit")
      (`PaperFlipbookComponent.SetLooping` (`self.Sprite`) false))))

(event `self.Sprite.OnFinishedPlaying`
  (bind _sprite (`self.Sprite`))
  ; On Sprite finish playing
  ;; Check Snail != dead
  (if (not (`self.IsDead`))
    ;; After hit animation finishes playing, Snail is no longer receiving damage, reset flipbook animation to walk, reset looping to true and call Play node on sprite component
    (set `self.IsReceivingDamage` false)
    (`PaperFlipbookComponent.SetFlipbook` _sprite "/Game/Assets/Mobs/Snail/Flipbooks/FB_Snail_Walk.FB_Snail_Walk")
    (`PaperFlipbookComponent.SetLooping` _sprite true)
    (`PaperFlipbookComponent.Play` _sprite)))

(event `self.EnemyDetector.OnComponentBeginOverlap`
  (params (OverlappedComponent :type "PrimitiveComponent Object Reference") (OtherActor :type "Actor Object Reference") (OtherComp :type "PrimitiveComponent Object Reference") (OtherBodyIndex :type Integer) (bFromSweep :type Boolean) (SweepResult :type "HitResult Structure (by ref)"))
  ; BP_Enemy Detection
  (for _array_element (`PrimitiveComponent.GetOverlappingActors` (`self.EnemyDetector`) "/Game/Blueprints/BP_Enemy.BP_Enemy_C")
    (if (!= _array_element self)
      (`self.ChangeDirections`))))

(event `self.WallDetector.OnComponentBeginOverlap`
  (params (OverlappedComponent :type "PrimitiveComponent Object Reference") (OtherActor :type "Actor Object Reference") (OtherComp :type "PrimitiveComponent Object Reference") (OtherBodyIndex :type Integer) (bFromSweep :type Boolean) (SweepResult :type "HitResult Structure (by ref)"))
  ; Wall Detection
  (`self.ChangeDirections`))

(event `self.LedgeDetector.OnComponentEndOverlap`
  (params (OverlappedComponent :type "PrimitiveComponent Object Reference") (OtherActor :type "Actor Object Reference") (OtherComp :type "PrimitiveComponent Object Reference") (OtherBodyIndex :type Integer))
  ; Ledge Detection
  (`self.ChangeDirections`))

(event `self.CollisionSphere.OnComponentBeginOverlap`
  (params (OverlappedComponent :type "PrimitiveComponent Object Reference") (OtherActor :type "Actor Object Reference") (OtherComp :type "PrimitiveComponent Object Reference") (OtherBodyIndex :type Integer) (bFromSweep :type Boolean) (SweepResult :type "HitResult Structure (by ref)"))
  ; Snail and Player Collision Logic
  ;; Check Snail is NOT dead
  (if (not (`self.IsDead`))
    ;; If the actor that bumped into the snail is our BP_Character, apply damage to our BP_Character
    (if (== (`GameplayStatics.GetObjectClass` OtherActor) "/Game/Blueprints/BP_Character.BP_Character_C")
      (`/Engine/EditorBlueprintResources/StandardMacros.DoOnce` false :!label _label
        (:`Completed`
          (`GameplayStatics.ApplyDamage` OtherActor (`self.DamageAmount`) null self))))))

(event `self.CollisionSphere.OnComponentEndOverlap`
  (params (OverlappedComponent :type "PrimitiveComponent Object Reference") (OtherActor :type "Actor Object Reference") (OtherComp :type "PrimitiveComponent Object Reference") (OtherBodyIndex :type Integer))
  ; Snail and Player Collision Logic
  ;; Check Snail is NOT dead
  (if (not (`self.IsDead`))
    ;; If the actor that bumped into the snail is our BP_Character, apply damage to our BP_Character
    (if (== (`GameplayStatics.GetObjectClass` OtherActor) "/Game/Blueprints/BP_Character.BP_Character_C")
      (goto _label :!via `Reset`))))

(fn `ChangeDirections`
  (`self.K2_SetActorRotation` (`KismetMathLibrary.ComposeRotators` (`self.K2_GetActorRotation`) (struct :`Yaw` 180.0))))

(fn `EndHitstop`
  (set `self.CustomTimeDilation` 1.0))

(fn `EndSpriteFlickerEffect`
  ; With the Flicker Effect Timer reference, clear and invalidate the timer and set the sprite visibility to true
  (`KismetSystemLibrary.K2_ClearAndInvalidateTimerHandle` (`self.SpriteFlickerEffectTimer`))
  (`SceneComponent.SetVisibility` (`self.Sprite`) true false))

(fn `StartHitstop`
  (params (Duration :type "Float (single-precision)"))
  (set `self.CustomTimeDilation` 0.0)
  (`KismetSystemLibrary.K2_SetTimer` null "EndHitstop" Duration))

(fn `StartSpriteFlickerEffect`
  ; Create an event to call the ToggleSpriteFlickerEffect() by timer (every Flicker Interval)
  (bind _returnvalue (`KismetSystemLibrary.K2_SetTimerDelegate` (`|CreateDelegate` :!event `ToggleSpriteFlickerEffect`) (`self.FlickerInterval`) true))
  ; Save a reference to the return timer so we can stop the flicker effect
  (set `self.SpriteFlickerEffectTimer` _returnvalue))

(fn `ToggleSpriteFlickerEffect`
  (bind _sprite (`self.Sprite`))
  (`SceneComponent.SetVisibility` _sprite (not (`SceneComponent.bVisible` _sprite)) false))

(fn `UserConstructionScript`)